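; Football projectile for an accuracy mode, flung by touch through the AccuracyPawn and tracked by its camera.
; BeginPlay rolls random left/right wind bounded by game mode difficulty into the game state.
; Once flung, Tick applies that wind as an impulse and activates rotating movement.
; Any hit stops the spin, then after a delay has the pawn spawn a replacement and destroys the ball; field-goal scoring logic is left disconnected.
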(event `self.ReceiveBeginPlay`
  (`self.MakeWind`)
  (bind _asaccuracy_pawn (cast `/Game/Blueprints/AccuracyPawn` (`GameplayStatics.GetPlayerPawn` 0)))
  (set `self.As Accuracy Pawn` _asaccuracy_pawn)
  (set `self.Pawn` (`/Game/Blueprints/AccuracyPawn.TouchTest` _asaccuracy_pawn))
  (set `self.StartLoc` (`SceneComponent.K2_GetComponentLocation` (`self.StaticMeshComponent`)))
  (set `PlayerController.bEnableTouchOverEvents` true (`GameplayStatics.GetPlayerController` 0))
  (set `/Game/Blueprints/AccuracyPawn.FootballLoc` (`SceneComponent.K2_GetComponentToWorld` (`self.StaticMeshComponent`)) (`self.As Accuracy Pawn`)))

(event `self.StaticMeshComponent.OnInputTouchEnter`
  (params (FingerIndex :type "ETouchIndex Enum" :default "Touch1") (TouchedComponent :type "PrimitiveComponent Object Reference"))
  (`KismetSystemLibrary.PrintString` "Hello")
  (bind _output_get (set `TouchTest.FBIsHit` true (`self.Pawn`)))
  (`KismetSystemLibrary.PrintString` (`KismetStringLibrary.Conv_BoolToString` _output_get) true true (struct :`R` 0.250085 :`G` 1.0 :`B` 0.11 :`A` 1.0)))

(event `self.ReceiveTick`
  (params (DeltaSeconds :type "Float (single-precision)"))
  (`/Game/Blueprints/AccuracyPawn.CameraFollow` (`self.As Accuracy Pawn`) (`self.StaticMeshComponent`))
  (if (`TouchTest.bFlung` (`self.Pawn`))
    (`self.Wind`)
    (if (not (`self.Hit`))
      (`ActorComponent.Activate` (`self.RotatingMovement`) false))))

(event `self.StaticMeshComponent.OnComponentHit`
  (params (HitComponent :type "PrimitiveComponent Object Reference") (OtherActor :type "Actor Object Reference") (OtherComp :type "PrimitiveComponent Object Reference") (NormalImpulse :type "Vector Structure") (Hit :type "HitResult Structure (by ref)"))
  (bind _pawn (`self.Pawn`))
  (`ActorComponent.Deactivate` (`self.RotatingMovement`))
  (`KismetSystemLibrary.Delay` 2.0)
  (set `TouchTest.bFlung` false _pawn)
  (set `TouchTest.FBIsHit` false _pawn)
  (`/Game/Blueprints/AccuracyPawn.SpawnNewFootball` (`self.As Accuracy Pawn`))
  (`self.K2_DestroyActor`))

(event `self.StaticMeshComponent.OnComponentBeginOverlap`
  (params (OverlappedComponent :type "PrimitiveComponent Object Reference") (OtherActor :type "Actor Object Reference") (OtherComp :type "PrimitiveComponent Object Reference") (OtherBodyIndex :type Integer) (bFromSweep :type Boolean) (SweepResult :type "HitResult Structure (by ref)")))

(fn `MakeWind`
  (bind _asaccuracy_game_mode (cast `AccuracyGameMode` (`GameplayStatics.GetGameMode`)))
  (bind _asaccuracy_game_state (cast `AccuracyGameState` (`GameplayStatics.GetGameState`)))
  (if (`KismetMathLibrary.RandomBoolWithWeight` 0.5)
    (bind _returnvalue (mod (`KismetMathLibrary.RandomInteger` 1000) (+ (`AccuracyGameMode.GetDifficulty` _asaccuracy_game_mode) 1)))
    (`AccuracyGameState.SetWind` _asaccuracy_game_state (* _returnvalue -1))
    (else
      (`AccuracyGameState.SetWind` _asaccuracy_game_state _returnvalue))))

(fn `Reset`
  (bind _pawn (`self.Pawn`))
  (set `TouchTest.bFlung` false _pawn)
  (set `TouchTest.FBIsHit` false _pawn)
  (`/Game/Blueprints/DefaultPawn_BP.SpawnNewFootball` (`self.As Default Pawn BP`))
  (bind _returnvalue (`GameplayStatics.GetActorOfClass` "/Game/Blueprints/FG_GoodTrigger_BP.FG_GoodTrigger_BP_C"))
  (bind _nogoodright (`/Game/Blueprints/FG_GoodTrigger_BP.NoGoodRight` _returnvalue))
  (`ActorComponent.Activate` _nogoodright false)
  (bind _nogoodleft (`/Game/Blueprints/FG_GoodTrigger_BP.NoGoodLeft` _returnvalue))
  (`ActorComponent.Activate` _nogoodleft false)
  (bind _collisioncomponent (`TriggerBase.CollisionComponent` _returnvalue))
  (`ActorComponent.Activate` _collisioncomponent false)
  (`PrimitiveComponent.SetCollisionEnabled` _nogoodright "QueryOnly")
  (`PrimitiveComponent.SetCollisionEnabled` _nogoodleft "QueryOnly")
  (`PrimitiveComponent.SetCollisionEnabled` _collisioncomponent "QueryOnly")
  (`self.K2_DestroyActor`))

(fn `UserConstructionScript`)

(fn `Wind`
  (locals (WIndAmount :type Integer :default 0))
  (if (`self.Hit`)
    (`ActorComponent.Deactivate` (`self.RotatingMovement`))
    (else
      (bind _asaccuracy_game_state (cast `AccuracyGameState` (`GameplayStatics.GetGameState`)))
      (`PrimitiveComponent.AddImpulse` (`self.StaticMeshComponent`) (`KismetMathLibrary.MakeVector` (`KismetMathLibrary.Conv_IntToDouble` (`AccuracyGameState.GetWind` _asaccuracy_game_state))) "None" false))))