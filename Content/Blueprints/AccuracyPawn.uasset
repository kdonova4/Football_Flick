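; Player pawn for the football kicking accuracy mode, which sets up the HUD, footballs and saved high score.
; Tick samples touch Y movement for the TouchTest component, and CameraFollow eases position, aim and FOV after a flung ball.
; SpawnNewFootball picks a tagged yard line within the game mode's difficulty range, repositions the kick spot and spawns a ball.
; EndGame saves the high score and shows game over when no footballs remain.
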(event `self.ReceiveBeginPlay`
  (bind _touchtest (`self.TouchTest`))
  (bind _returnvalue (`GameplayStatics.DoesSaveGameExist` (`self.SlotName`)))
  (if _returnvalue
    (bind _returnvalue_2 (`GameplayStatics.LoadGameFromSlot` (`self.SlotName`)))
    (bind _output_get (set `self.AccuracySaveSubClass` _returnvalue_2))
    (bind _ashighest_accuracy_save (cast `/Game/Blueprints/HighestAccuracySave` _output_get))
    (bind _output_get_2 (set `self.HighScoreAccuracy` (`/Game/Blueprints/HighestAccuracySave.HighestAccuracy` _ashighest_accuracy_save)))
    (`KismetSystemLibrary.PrintString` (`KismetStringLibrary.Conv_IntToString` _output_get_2) true true (struct :`R` 0.041065 :`G` 1.0 :`A` 1.0)))
  (bind _outactors (`GameplayStatics.GetAllActorsOfClass` "/Game/Blueprints/YardLine_BP.YardLine_BP_C"))
  (set `self.Out Actors_0` _outactors)
  (bind _asaccuracy_game_mode (cast `AccuracyGameMode` (`GameplayStatics.GetGameMode`)))
  (set `self.As Accuracy Game Mode` _asaccuracy_game_mode)
  (set `AccuracyGameMode.PC` (`GameplayStatics.GetPlayerController` 0) _asaccuracy_game_mode)
  (bind _returnvalue_3 (`|CreateWidget` "/Game/Blueprints/AccuracyUI.AccuracyUI_C"))
  (bind _output_get_3 (set `self.UI` _returnvalue_3))
  (`/Game/Blueprints/AccuracyUI.SetFooballs` _output_get_3)
  (`/Game/Blueprints/AccuracyUI.SetAccuracy` _output_get_3)
  (`UserWidget.AddToViewport` _output_get_3 0)
  (bind _output_get_4 (set `self.Rotation` (`KismetMathLibrary.MakeRotator` 90.0 -70.0 90.0)))
  (`|SpawnActorFromClass` "/Game/Blueprints/AccuracyFootball_Blueprint.AccuracyFootball_Blueprint_C" (`KismetMathLibrary.MakeTransform` (`SceneComponent.K2_GetComponentLocation` (`self.Scene1`)) _output_get_4) "Undefined" "OverrideRootScale" null null)
  (set `self.NewVar_0` null)
  (set `TouchTest.MyCurve` "/Game/Blueprints/KickAngle.KickAngle" _touchtest)
  (set `TouchTest.MyCurvePower` "/Game/Blueprints/KickPower.KickPower" _touchtest)
  (set `self.CamLoc` (`SceneComponent.K2_GetComponentToWorld` (`self.Camera`))))

(event `CameraFollow`
  (params (Football :type "StaticMeshComponent Object Reference"))
  (bind (_camloc_location _camloc_rotation) (`KismetMathLibrary.BreakTransform` (`self.CamLoc`)))
  (bind _camera (`self.Camera`))
  (bind _returnvalue (`SceneComponent.K2_GetComponentLocation` _camera))
  (bind _returnvalue_location (`KismetMathLibrary.BreakTransform` (`KismetMathLibrary.TInterpTo` (`KismetMathLibrary.MakeTransform` _returnvalue) (`KismetMathLibrary.MakeTransform` (`SceneComponent.K2_GetComponentLocation` (`self.Scene`))) (`GameplayStatics.GetWorldDeltaSeconds`) 1.0)))
  (if (`TouchTest.bFlung` (`self.TouchTest`))
    (`SceneComponent.K2_SetWorldLocationAndRotation` _camera _returnvalue_location (`KismetMathLibrary.RInterpTo` (`SceneComponent.K2_GetComponentRotation` _camera) (`KismetMathLibrary.FindLookAtRotation` _returnvalue (`SceneComponent.K2_GetComponentLocation` Football)) (`GameplayStatics.GetWorldDeltaSeconds`) 2.0) false false)
    (bind (_direction _newtrack_0) (`Timeline|Alpha` :!label _label)
      (:`Update`
        (`CameraComponent.SetFieldOfView` (`self.Camera`) (`|EaseFunction` "EaseInOut" _newtrack_0 (`self.FOV`) 35.0))))
    (else
      (`CameraComponent.SetFieldOfView` (`self.Camera`) (`self.FOV`))
      (`SceneComponent.K2_SetWorldLocationAndRotation` _camera _camloc_location _camloc_rotation false false)
      (goto _label :!via `SetNewTime`))))

(event `self.ReceiveTick`
  (params (DeltaSeconds :type "Float (single-precision)"))
  (bind _touchtest (`self.TouchTest`))
  (bind (_locationx _locationy) (`PlayerController.GetInputTouchState` (`GameplayStatics.GetPlayerController` 0) "Touch1"))
  (`|ExecutionSequence`
    (:`then_0`
      (set `TouchTest.YVeloOld` _locationy _touchtest)
      (`KismetSystemLibrary.Delay` 0.02)
      (set `TouchTest.YVeloNew` _locationy _touchtest))
    (:`then_1`
      (set `TouchTest.YDiff` (- (`TouchTest.YVeloOld` _touchtest) (`TouchTest.YVeloNew` _touchtest)) _touchtest))))

(event `SpawnNewFootball`
  (bind _as_accuracy_game_mode (`self.As Accuracy Game Mode`))
  (bind (_returnvalue_x _returnvalue_y _returnvalue_z) (`KismetMathLibrary.BreakVector` (`SceneComponent.K2_GetComponentLocation` (`StaticMeshActor.StaticMeshComponent` (`self.YardLineSpawn`)))))
  (`/Engine/EditorBlueprintResources/StandardMacros.IncrementInt` (`self.Count`)
    (:`  `
      (bind _output_get (set `self.Tag` (`KismetStringLibrary.Conv_StringToName` (`KismetStringLibrary.Conv_IntToString` (`KismetMathLibrary.RandomIntegerInRange` (`AccuracyGameMode.GetDifficultyFloor` _as_accuracy_game_mode) (`KismetMathLibrary.Clamp` (`AccuracyGameMode.GetDifficulty` _as_accuracy_game_mode) 0 36))))))
      (`KismetSystemLibrary.PrintString` (`KismetStringLibrary.Conv_NameToString` _output_get) true true (struct :`R` 1.0 :`G` 0.232749 :`A` 1.0))
      (`self.EndGame`)
      (for _array_element (`self.Out Actors_0`)
        (if (`self.ActorHasTag` _array_element (`self.Tag`))
          (bind _output_get_2 (set `self.YardLineSpawn` _array_element))))
      (`KismetSystemLibrary.PrintString` (`KismetSystemLibrary.GetObjectName` _output_get_2) true true (struct :`R` 0.064623 :`B` 1.0 :`A` 1.0))
      (`SceneComponent.K2_SetWorldLocation` (`self.Scene2`) (`KismetMathLibrary.MakeVector` (`KismetMathLibrary.RandomFloatInRange` -71.0 455.0) _returnvalue_y _returnvalue_z) false false)
      (set `self.CamLoc` (`SceneComponent.K2_GetComponentToWorld` (`self.Scene3`)))
      (`|SpawnActorFromClass` "/Game/Blueprints/AccuracyFootball_Blueprint.AccuracyFootball_Blueprint_C" (`KismetMathLibrary.MakeTransform` (`SceneComponent.K2_GetComponentLocation` (`self.Scene1`)) (`self.Rotation`)) "Undefined" "OverrideRootScale" null null)
      (set `self.NewVar_0` null))))

(event `Key|SpaceBar`
  (params (Key :type "Key Structure"))
  (bind _touchtest (`self.TouchTest`))
  (:`Pressed`
    (set `TouchTest.bFlung` true _touchtest))
  (:`Released`
    (set `TouchTest.bFlung` false _touchtest)))

(event `Key|F`
  (params (Key :type "Key Structure"))
  (:`Pressed`
    (bind _outactors (`GameplayStatics.GetAllActorsOfClass` "/Game/Blueprints/Football_Blueprint.Football_Blueprint_C"))
    (`self.K2_DestroyActor` _outactors))
  (:`Released`
    (`|SpawnActorFromClass` "/Game/Blueprints/Football_Blueprint.Football_Blueprint_C" (`KismetMathLibrary.MakeTransform` (`SceneComponent.K2_GetComponentLocation` (`self.Scene1`)) (`self.Rotation`)) "Undefined" "OverrideRootScale" null null)))

(fn `EndGame`
  (bind _asaccuracy_game_mode (cast `AccuracyGameMode` (`GameplayStatics.GetGameMode`)))
  (if (<= (`AccuracyGameMode.GetFootballsLeft` _asaccuracy_game_mode) 0)
    (bind _returnvalue (`GameplayStatics.DoesSaveGameExist` (`self.SlotName`)))
    (if _returnvalue
      (bind _returnvalue_2 (`GameplayStatics.LoadGameFromSlot` (`self.SlotName`)))
      (bind _output_get (set `self.AccuracySaveSubClass` _returnvalue_2))
      (bind _ashighest_accuracy_save (cast `/Game/Blueprints/HighestAccuracySave` _output_get))
      (if (<= (`/Game/Blueprints/HighestAccuracySave.HighestAccuracy` _ashighest_accuracy_save) (`self.HighScoreAccuracy`))
        (set `/Game/Blueprints/HighestAccuracySave.HighestAccuracy` (`self.HighScoreAccuracy`) _ashighest_accuracy_save)
        (`GameplayStatics.SaveGameToSlot` (`self.AccuracySaveSubClass`) (`self.SlotName`)))
      (else
        (bind _returnvalue_3 (`GameplayStatics.CreateSaveGameObject` "/Game/Blueprints/HighestAccuracySave.HighestAccuracySave_C"))
        (bind _output_get_2 (set `self.AccuracySaveSubClass` _returnvalue_3))
        (bind _ashighest_accuracy_save_2 (cast `/Game/Blueprints/HighestAccuracySave` _output_get_2))
        (if (<= (`/Game/Blueprints/HighestAccuracySave.HighestAccuracy` _ashighest_accuracy_save_2) (`self.HighScoreAccuracy`))
          (set `/Game/Blueprints/HighestAccuracySave.HighestAccuracy` (`self.HighScoreAccuracy`) _ashighest_accuracy_save_2)
          (`GameplayStatics.SaveGameToSlot` (`self.AccuracySaveSubClass`) (`self.SlotName`)))))
    (`Widget.RemoveFromParent` (`self.UI`))
    (bind _returnvalue_4 (`|CreateWidget` "/Game/Blueprints/AccuracyUI_GameOver.AccuracyUI_GameOver_C"))
    (`UserWidget.AddToViewport` _returnvalue_4 0)
    (`AccuracyGameMode.PauseGame` _asaccuracy_game_mode)))

(fn `UserConstructionScript`)