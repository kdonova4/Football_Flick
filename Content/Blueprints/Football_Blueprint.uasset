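; Football actor for an endless, touch-controlled field goal game, handling one kick from spawn to replacement.
; BeginPlay rolls difficulty-scaled wind into the game state and flags touches on the pawn.
; While flung, Tick applies wind as a sideways X impulse and spins the ball until it hits, with the camera following throughout.
; Trigger overlaps or floor hits update score, balls and UI, and landing spawns a new ball before destroying this one.
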(event `self.ReceiveBeginPlay`
  (`self.MakeWind`)
  (bind _asdefault_pawn_bp (cast `/Game/Blueprints/DefaultPawn_BP` (`GameplayStatics.GetPlayerPawn` 0)))
  (set `self.As Default Pawn BP` _asdefault_pawn_bp)
  (set `self.Pawn` (`/Game/Blueprints/DefaultPawn_BP.TouchTest` _asdefault_pawn_bp))
  (set `self.StartLoc` (`SceneComponent.K2_GetComponentLocation` (`self.StaticMeshComponent`)))
  (set `PlayerController.bEnableTouchOverEvents` true (`GameplayStatics.GetPlayerController` 0))
  (set `/Game/Blueprints/DefaultPawn_BP.FootballLoc` (`SceneComponent.K2_GetComponentToWorld` (`self.StaticMeshComponent`)) (`self.As Default Pawn BP`)))

(event `self.StaticMeshComponent.OnInputTouchEnter`
  (params (FingerIndex :type "ETouchIndex Enum" :default "Touch1") (TouchedComponent :type "PrimitiveComponent Object Reference"))
  (`KismetSystemLibrary.PrintString` "Hello")
  (bind _output_get (set `TouchTest.FBIsHit` true (`self.Pawn`)))
  (`KismetSystemLibrary.PrintString` (`KismetStringLibrary.Conv_BoolToString` _output_get) true true (struct :`R` 0.250085 :`G` 1.0 :`B` 0.11 :`A` 1.0)))

(event `self.ReceiveTick`
  (params (DeltaSeconds :type "Float (single-precision)"))
  (`/Game/Blueprints/DefaultPawn_BP.CameraFollow` (`self.As Default Pawn BP`) (`self.StaticMeshComponent`))
  (if (`TouchTest.bFlung` (`self.Pawn`))
    (`self.Wind`)
    (if (not (`self.Hit`))
      (`ActorComponent.Activate` (`self.RotatingMovement`) false))))

(event `self.StaticMeshComponent.OnComponentHit`
  (params (HitComponent :type "PrimitiveComponent Object Reference") (OtherActor :type "Actor Object Reference") (OtherComp :type "PrimitiveComponent Object Reference") (NormalImpulse :type "Vector Structure") (Hit :type "HitResult Structure (by ref)"))
  (bind _pawn (`self.Pawn`))
  (bind _ui (`/Game/Blueprints/DefaultPawn_BP.UI` (`self.As Default Pawn BP`)))
  (set `self.Hit` true)
  (if (`KismetStringLibrary.EqualEqual_StrStr` (`KismetSystemLibrary.GetObjectName` OtherActor) "Floor")
    (if (or (`self.FgGood`) (`self.FgNoGood`))
      _
      (elif (not (`self.FgHitGround`))
        (set `self.FgHitGround` true)
        (set `self.StreakCount` 1)
        (bind _returnvalue (`GameplayStatics.GetActorOfClass` "/Game/Blueprints/FG_GoodTrigger_BP.FG_GoodTrigger_BP_C"))
        (`/Game/Blueprints/FG_GoodTrigger_BP.DecreaseBalls` _returnvalue)
        (`/Game/Blueprints/EndlessUI.SetFooballs` _ui)
        (`/Game/Blueprints/EndlessUI.SetScore` _ui)))
    (`KismetSystemLibrary.PrintString` (`KismetStringLibrary.Conv_DoubleToString` (`KismetMathLibrary.Vector_Distance` (`self.StartLoc`) (`SceneComponent.K2_GetComponentLocation` (`self.StaticMeshComponent`)))))
    (`ActorComponent.Deactivate` (`self.RotatingMovement`))
    (`KismetSystemLibrary.Delay` 2.0)
    (set `TouchTest.bFlung` false _pawn)
    (set `TouchTest.FBIsHit` false _pawn)
    (`/Game/Blueprints/DefaultPawn_BP.SpawnNewFootball` (`self.As Default Pawn BP`))
    (`self.K2_DestroyActor`)))

(event `self.StaticMeshComponent.OnComponentBeginOverlap`
  (params (OverlappedComponent :type "PrimitiveComponent Object Reference") (OtherActor :type "Actor Object Reference") (OtherComp :type "PrimitiveComponent Object Reference") (OtherBodyIndex :type Integer) (bFromSweep :type Boolean) (SweepResult :type "HitResult Structure (by ref)"))
  (bind _ui (`/Game/Blueprints/DefaultPawn_BP.UI` (`self.As Default Pawn BP`)))
  (bind _ui_2 (`/Game/Blueprints/DefaultPawn_BP.UI` (`self.As Default Pawn BP`)))
  (if (`KismetStringLibrary.EqualEqual_StrStr` (`KismetSystemLibrary.GetObjectName` OtherActor) "FG_GoodTrigger_BP")
    (bind _returnvalue (`GameplayStatics.GetActorOfClass` "/Game/Blueprints/FG_GoodTrigger_BP.FG_GoodTrigger_BP_C"))
    (if (not (`self.FgNoGood`))
      (set `self.FgGood` true)
      (`/Game/Blueprints/FG_GoodTrigger_BP.IncreaseScore` _returnvalue)
      (`/Game/Blueprints/EndlessUI.SetFooballs` _ui)
      (`/Game/Blueprints/EndlessUI.SetScore` _ui))
    (else
      (bind _returnvalue_2 (`GameplayStatics.GetActorOfClass` "/Game/Blueprints/FG_GoodTrigger_BP.FG_GoodTrigger_BP_C"))
      (if (not (`self.FgGood`))
        (set `self.FgNoGood` true)
        (set `/Game/Blueprints/FG_GoodTrigger_BP.Streak` 1 _returnvalue_2)
        (`/Game/Blueprints/FG_GoodTrigger_BP.DecreaseBalls` _returnvalue_2)
        (`/Game/Blueprints/EndlessUI.SetFooballs` _ui_2)
        (`/Game/Blueprints/EndlessUI.SetScore` _ui_2)))))

(fn `MakeWind`
  (bind _asendless_game_mode (cast `EndlessGameMode` (`GameplayStatics.GetGameMode`)))
  (bind _asendless_game_state (cast `EndlessGameState` (`GameplayStatics.GetGameState`)))
  (if (`KismetMathLibrary.RandomBoolWithWeight` 0.5)
    (bind _returnvalue (mod (`KismetMathLibrary.RandomInteger` 1000) (+ (`EndlessGameMode.GetDifficulty` _asendless_game_mode) 1)))
    (`EndlessGameState.SetWind` _asendless_game_state (* _returnvalue -1))
    (else
      (`EndlessGameState.SetWind` _asendless_game_state _returnvalue))))

(fn `UserConstructionScript`)

(fn `Wind`
  (locals (WIndAmount :type Integer :default 0))
  (if (`self.Hit`)
    (`ActorComponent.Deactivate` (`self.RotatingMovement`))
    (else
      (bind _asendless_game_state (cast `EndlessGameState` (`GameplayStatics.GetGameState`)))
      (`PrimitiveComponent.AddImpulse` (`self.StaticMeshComponent`) (`KismetMathLibrary.MakeVector` (`KismetMathLibrary.Conv_IntToDouble` (`EndlessGameState.GetWind` _asendless_game_state))) "None" false))))