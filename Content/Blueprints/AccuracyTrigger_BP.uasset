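; Goal trigger that scores footballs in the accuracy game mode.
; Middle100's overlap sorts airborne balls by X into five point bands or a miss, flashes the band's GoalBox widget on a score, spawns a mark, then resets the ball.
; Scores and misses update average accuracy, balls left and pawn UI; scores also raise difficulty, with SetDifficultyLimit stepping its floor except on Left 50.
; Other zone overlaps are empty; high-score saving is disconnected.
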(event `self.ReceiveBeginPlay`
  (bind _asaccuracy_game_mode (cast `AccuracyGameMode` (`GameplayStatics.GetGameMode`)))
  (set `self.As Accuracy Game Mode` _asaccuracy_game_mode)
  (`KismetSystemLibrary.PrintString` (`KismetStringLibrary.Conv_VectorToString` (`KismetSystemLibrary.GetComponentBounds` (`self.Middle100`))))
  (bind _asaccuracy_pawn (cast `/Game/Blueprints/AccuracyPawn` (`GameplayStatics.GetPlayerPawn` 0)))
  (set `self.As Accuracy Pawn` _asaccuracy_pawn))

(event `self.Right50.OnComponentBeginOverlap`
  (params (OverlappedComponent :type "PrimitiveComponent Object Reference") (OtherActor :type "Actor Object Reference") (OtherComp :type "PrimitiveComponent Object Reference") (OtherBodyIndex :type Integer) (bFromSweep :type Boolean) (SweepResult :type "HitResult Structure (by ref)")))

(event `self.Right75.OnComponentBeginOverlap`
  (params (OverlappedComponent :type "PrimitiveComponent Object Reference") (OtherActor :type "Actor Object Reference") (OtherComp :type "PrimitiveComponent Object Reference") (OtherBodyIndex :type Integer) (bFromSweep :type Boolean) (SweepResult :type "HitResult Structure (by ref)")))

(event `self.Middle100.OnComponentBeginOverlap`
  (params (OverlappedComponent :type "PrimitiveComponent Object Reference") (OtherActor :type "Actor Object Reference") (OtherComp :type "PrimitiveComponent Object Reference") (OtherBodyIndex :type Integer) (bFromSweep :type Boolean) (SweepResult :type "HitResult Structure (by ref)"))
  (bind _returnvalue_x (`KismetMathLibrary.BreakVector` (`self.K2_GetActorLocation` OtherActor)))
  (bind _returnvalue (`self.K2_GetActorLocation` OtherActor))
  (bind _asaccuracy_football_blueprint (cast `/Game/Blueprints/AccuracyFootball_Blueprint` OtherActor))
  (if (not (`/Game/Blueprints/AccuracyFootball_Blueprint.HitGround` _asaccuracy_football_blueprint))
    (set `/Game/Blueprints/AccuracyFootball_Blueprint.Hit` true _asaccuracy_football_blueprint)
    (`KismetSystemLibrary.PrintString` "OVERLAPPED" true true (struct :`R` 0.340665 :`G` 1.0 :`A` 1.0))
    (if (and (<= _returnvalue_x 460.0) (>= _returnvalue_x 352.600006))
      (`/Engine/EditorBlueprintResources/StandardMacros.DoOnce` false :!label _label
        (:`Completed`
          (`KismetSystemLibrary.PrintString` "Left 50")
          (`self.IncreaseAccuracy` 50)
          (bind _asgoal_box (cast `/Game/Blueprints/GoalBox` (`WidgetComponent.GetWidget` (`self.Widget4`))))
          (`UserWidget.PlayAnimation` _asgoal_box (`/Game/Blueprints/GoalBox.Fadeinout` _asgoal_box) 0.0 1 "Forward" 1.0 false)
          (`|SpawnActorFromClass` "/Game/Blueprints/Football/GoodMark.GoodMark_C" (`KismetMathLibrary.MakeTransform` _returnvalue) "Undefined" "OverrideRootScale" null null)
          (`KismetSystemLibrary.Delay` 1.0)
          (`/Game/Blueprints/AccuracyFootball_Blueprint.ResetAccuracy` _asaccuracy_football_blueprint)
          (goto _label :!via `Reset`)))
      (elif (and (< _returnvalue_x 352.600006) (>= _returnvalue_x 245.199997))
        (`/Engine/EditorBlueprintResources/StandardMacros.DoOnce` false :!label _label_2
          (:`Completed`
            (`KismetSystemLibrary.PrintString` "left 75")
            (`self.IncreaseAccuracy` 75)
            (`self.SetDifficultyLimit`)
            (bind _asgoal_box_2 (cast `/Game/Blueprints/GoalBox` (`WidgetComponent.GetWidget` (`self.Widget3`))))
            (`UserWidget.PlayAnimation` _asgoal_box_2 (`/Game/Blueprints/GoalBox.Fadeinout` _asgoal_box_2) 0.0 1 "Forward" 1.0 false)
            (`|SpawnActorFromClass` "/Game/Blueprints/Football/GoodMark.GoodMark_C" (`KismetMathLibrary.MakeTransform` _returnvalue) "Undefined" "OverrideRootScale" null null)
            (`KismetSystemLibrary.Delay` 1.0)
            (`/Game/Blueprints/AccuracyFootball_Blueprint.ResetAccuracy` _asaccuracy_football_blueprint)
            (goto _label_2 :!via `Reset`)))
        (elif (and (< _returnvalue_x 245.199997) (>= _returnvalue_x 137.800003))
          (`/Engine/EditorBlueprintResources/StandardMacros.DoOnce` false :!label _label_3
            (:`Completed`
              (`KismetSystemLibrary.PrintString` "Middle 100")
              (`self.IncreaseAccuracy` 100)
              (`self.SetDifficultyLimit`)
              (bind _asgoal_box_3 (cast `/Game/Blueprints/GoalBox` (`WidgetComponent.GetWidget` (`self.Widget2`))))
              (`UserWidget.PlayAnimation` _asgoal_box_3 (`/Game/Blueprints/GoalBox.Fadeinout` _asgoal_box_3) 0.0 1 "Forward" 1.0 false)
              (`|SpawnActorFromClass` "/Game/Blueprints/Football/GoodMark.GoodMark_C" (`KismetMathLibrary.MakeTransform` _returnvalue) "Undefined" "OverrideRootScale" null null)
              (`KismetSystemLibrary.Delay` 1.0)
              (`/Game/Blueprints/AccuracyFootball_Blueprint.ResetAccuracy` _asaccuracy_football_blueprint)
              (goto _label_3 :!via `Reset`)))
          (elif (and (< _returnvalue_x 137.800003) (>= _returnvalue_x 29.6))
            (`/Engine/EditorBlueprintResources/StandardMacros.DoOnce` false :!label _label_4
              (:`Completed`
                (`KismetSystemLibrary.PrintString` "Right 75")
                (`self.IncreaseAccuracy` 75)
                (`self.SetDifficultyLimit`)
                (bind _asgoal_box_4 (cast `/Game/Blueprints/GoalBox` (`WidgetComponent.GetWidget` (`self.Widget1`))))
                (`UserWidget.PlayAnimation` _asgoal_box_4 (`/Game/Blueprints/GoalBox.Fadeinout` _asgoal_box_4) 0.0 1 "Forward" 1.0 false)
                (`|SpawnActorFromClass` "/Game/Blueprints/Football/GoodMark.GoodMark_C" (`KismetMathLibrary.MakeTransform` _returnvalue) "Undefined" "OverrideRootScale" null null)
                (`KismetSystemLibrary.Delay` 1.0)
                (`/Game/Blueprints/AccuracyFootball_Blueprint.ResetAccuracy` _asaccuracy_football_blueprint)
                (goto _label_4 :!via `Reset`)))
            (elif (and (< _returnvalue_x 29.6) (>= _returnvalue_x -77.800003))
              (`/Engine/EditorBlueprintResources/StandardMacros.DoOnce` false :!label _label_5
                (:`Completed`
                  (`KismetSystemLibrary.PrintString` "Right 50")
                  (`self.IncreaseAccuracy` 50)
                  (`self.SetDifficultyLimit`)
                  (bind _asgoal_box_5 (cast `/Game/Blueprints/GoalBox` (`WidgetComponent.GetWidget` (`self.Widget`))))
                  (`UserWidget.PlayAnimation` _asgoal_box_5 (`/Game/Blueprints/GoalBox.Fadeinout` _asgoal_box_5) 0.0 1 "Forward" 1.0 false)
                  (`|SpawnActorFromClass` "/Game/Blueprints/Football/GoodMark.GoodMark_C" (`KismetMathLibrary.MakeTransform` _returnvalue) "Undefined" "OverrideRootScale" null null)
                  (`KismetSystemLibrary.Delay` 1.0)
                  (`/Game/Blueprints/AccuracyFootball_Blueprint.ResetAccuracy` _asaccuracy_football_blueprint)
                  (goto _label_5 :!via `Reset`)))
              (elif (or (> _returnvalue_x 460.0) (< _returnvalue_x -77.800003))
                (`/Engine/EditorBlueprintResources/StandardMacros.DoOnce` false :!label _label_6
                  (:`Completed`
                    (`KismetSystemLibrary.PrintString` "MISS")
                    (`self.DecreaseBalls` 0)
                    (`|SpawnActorFromClass` "/Game/Blueprints/Football/NoGoodMark.NoGoodMark_C" (`KismetMathLibrary.MakeTransform` _returnvalue) "Undefined" "OverrideRootScale" null null)
                    (`KismetSystemLibrary.Delay` 1.0)
                    (`/Game/Blueprints/AccuracyFootball_Blueprint.ResetAccuracy` _asaccuracy_football_blueprint)
                    (goto _label_6 :!via `Reset`)))))))))))

(event `self.Left75.OnComponentBeginOverlap`
  (params (OverlappedComponent :type "PrimitiveComponent Object Reference") (OtherActor :type "Actor Object Reference") (OtherComp :type "PrimitiveComponent Object Reference") (OtherBodyIndex :type Integer) (bFromSweep :type Boolean) (SweepResult :type "HitResult Structure (by ref)")))

(event `self.Left50.OnComponentBeginOverlap`
  (params (OverlappedComponent :type "PrimitiveComponent Object Reference") (OtherActor :type "Actor Object Reference") (OtherComp :type "PrimitiveComponent Object Reference") (OtherBodyIndex :type Integer) (bFromSweep :type Boolean) (SweepResult :type "HitResult Structure (by ref)")))

(event `self.Middle100.OnComponentHit`
  (params (HitComponent :type "PrimitiveComponent Object Reference") (OtherActor :type "Actor Object Reference") (OtherComp :type "PrimitiveComponent Object Reference") (NormalImpulse :type "Vector Structure") (Hit :type "HitResult Structure (by ref)"))
  (`KismetSystemLibrary.PrintString` "HITTING")
  (`self.IncreaseAccuracy` 100))

(fn `DecreaseBalls`
  (params (`Accuracy Num` :type Integer))
  (bind _asaccuracy_game_mode (cast `AccuracyGameMode` (`GameplayStatics.GetGameMode`)))
  (bind _returnvalue (`AccuracyGameMode.SetTotalAccuracy` _asaccuracy_game_mode (+ (`AccuracyGameMode.GetTotalAccuracy` _asaccuracy_game_mode) `Accuracy Num`)))
  (bind _asaccuracy_pawn (cast `/Game/Blueprints/AccuracyPawn` (`GameplayStatics.GetPlayerPawn` 0)))
  (`AccuracyGameMode.SetAccuracy` _asaccuracy_game_mode (/ _returnvalue (`/Game/Blueprints/AccuracyPawn.Count` _asaccuracy_pawn)))
  (bind _result (`/Engine/EditorBlueprintResources/StandardMacros.DecrementInt` (`AccuracyGameMode.GetFootballsLeft` _asaccuracy_game_mode))
    (:`  `
      (`AccuracyGameMode.SetFootballsLeft` _asaccuracy_game_mode _result)
      (bind _ui (`/Game/Blueprints/AccuracyPawn.UI` _asaccuracy_pawn))
      (`/Game/Blueprints/AccuracyUI.SetAccuracy` _ui)
      (`/Game/Blueprints/AccuracyUI.SetFooballs` _ui)
      (`KismetSystemLibrary.PrintString` (`KismetStringLibrary.Conv_IntToString` (`AccuracyGameMode.GetFootballsLeft` _asaccuracy_game_mode))))))

(fn `IncreaseAccuracy`
  (params (AccuracyNum :type Integer))
  (bind _as_accuracy_game_mode (`self.As Accuracy Game Mode`))
  (bind _as_accuracy_game_mode_2 (`self.As Accuracy Game Mode`))
  (bind _returnvalue (`AccuracyGameMode.GetDifficulty` _as_accuracy_game_mode))
  (`KismetSystemLibrary.PrintString` (`KismetStringLibrary.Conv_IntToString` _returnvalue) true true (struct :`R` 0.074377 :`B` 1.0 :`A` 1.0))
  (bind _result (`/Engine/EditorBlueprintResources/StandardMacros.IncrementInt` _returnvalue)
    (:`  `
      (`AccuracyGameMode.SetDifficulty` _as_accuracy_game_mode _result)
      (bind _returnvalue_2 (`AccuracyGameMode.SetTotalAccuracy` _as_accuracy_game_mode (+ AccuracyNum (`AccuracyGameMode.GetTotalAccuracy` _as_accuracy_game_mode))))
      (bind _asaccuracy_pawn (cast `/Game/Blueprints/AccuracyPawn` (`GameplayStatics.GetPlayerPawn` 0)))
      (`AccuracyGameMode.SetAccuracy` _as_accuracy_game_mode (/ _returnvalue_2 (`/Game/Blueprints/AccuracyPawn.Count` _asaccuracy_pawn)))
      (bind _ui (`/Game/Blueprints/AccuracyPawn.UI` _asaccuracy_pawn))
      (`/Game/Blueprints/AccuracyUI.SetAccuracy` _ui)
      (bind _result_2 (`/Engine/EditorBlueprintResources/StandardMacros.DecrementInt` (`AccuracyGameMode.GetFootballsLeft` _as_accuracy_game_mode_2))
        (:`  `
          (`AccuracyGameMode.SetFootballsLeft` _as_accuracy_game_mode_2 _result_2)
          (`/Game/Blueprints/AccuracyUI.SetFooballs` _ui)
          (set `/Game/Blueprints/AccuracyPawn.HighScoreAccuracy` (`AccuracyGameMode.GetAccuracy` (`self.As Accuracy Game Mode`)) (`self.As Accuracy Pawn`)))))))

(fn `SetDifficultyLimit`
  (bind _as_accuracy_game_mode (`self.As Accuracy Game Mode`))
  (if (== (- (`AccuracyGameMode.GetDifficulty` _as_accuracy_game_mode) (`AccuracyGameMode.GetDifficultyFloor` _as_accuracy_game_mode)) 10)
    (`AccuracyGameMode.SetDifficultyFloor` (`self.As Accuracy Game Mode`) (+ (`AccuracyGameMode.GetDifficultyFloor` (`self.As Accuracy Game Mode`)) 5))
    (`KismetSystemLibrary.PrintString` "RESET NEW LIMIT")))

(fn `UserConstructionScript`)