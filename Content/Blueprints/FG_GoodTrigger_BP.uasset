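; Field goal trigger that judges kicked footballs as good or no good in the endless game mode.
; The first overlap disables the center and two side zones; an airborne ball gets a result marker and a delayed reset.
; Goals add streak-multiplied score, raise difficulty and its stepped floor, and save high scores to a ScoreSave slot.
; Misses reset the streak and remove a football, with the pawn's UI updated either way.
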(event `self.ReceiveBeginPlay`
  (bind _asendless_game_mode (cast `EndlessGameMode` (`GameplayStatics.GetGameMode`)))
  (set `self.As Endless Game Mode` _asendless_game_mode)
  (bind _asdefault_pawn_bp (cast `/Game/Blueprints/DefaultPawn_BP` (`GameplayStatics.GetPlayerPawn` 0)))
  (set `self.As Default Pawn BP` _asdefault_pawn_bp))

(event `self.ReceiveActorBeginOverlap`
  (params (OtherActor :type "Actor Object Reference")))

(event `self.CollisionComponent.OnComponentBeginOverlap`
  (params (OverlappedComponent :type "PrimitiveComponent Object Reference") (OtherActor :type "Actor Object Reference") (OtherComp :type "PrimitiveComponent Object Reference") (OtherBodyIndex :type Integer) (bFromSweep :type Boolean) (SweepResult :type "HitResult Structure (by ref)"))
  (`PrimitiveComponent.SetCollisionEnabled` (`self.CollisionComponent`) "NoCollision")
  (`PrimitiveComponent.SetCollisionEnabled` (`self.NoGoodRight`) "NoCollision")
  (`PrimitiveComponent.SetCollisionEnabled` (`self.NoGoodLeft`) "NoCollision")
  (`ActorComponent.Deactivate` (`self.CollisionComponent`))
  (`ActorComponent.Deactivate` OverlappedComponent)
  (`ActorComponent.Deactivate` (`self.NoGoodLeft`))
  (`ActorComponent.Deactivate` (`self.NoGoodRight`))
  (bind _asfootball_blueprint (cast `/Game/Blueprints/Football_Blueprint` OtherActor))
  (if (not (`/Game/Blueprints/Football_Blueprint.FgHitGround` _asfootball_blueprint))
    (set `/Game/Blueprints/Football_Blueprint.FgGood` true _asfootball_blueprint)
    (`|SpawnActorFromClass` "/Game/Blueprints/Football/GoodMark.GoodMark_C" (`KismetMathLibrary.MakeTransform` (`self.K2_GetActorLocation` OtherActor)) "Undefined" "OverrideRootScale" null null)
    (`self.SetDifficultyLimit`)
    (bind _asfootball_blueprint_2 (cast `/Game/Blueprints/Football_Blueprint` OtherActor))
    (set `/Game/Blueprints/Football_Blueprint.FgGood` true _asfootball_blueprint_2)
    (`self.IncreaseScore`)
    (`/Game/Blueprints/EndlessUI.SetScore` (`/Game/Blueprints/DefaultPawn_BP.UI` (`self.As Default Pawn BP`)))
    (bind _asfootball_blueprint_3 (cast `/Game/Blueprints/Football_Blueprint` OtherActor))
    (`KismetSystemLibrary.Delay` 2.0)
    (`/Game/Blueprints/Football_Blueprint.Reset` _asfootball_blueprint_3)))

(event `self.NoGoodLeft.OnComponentBeginOverlap`
  (params (OverlappedComponent :type "PrimitiveComponent Object Reference") (OtherActor :type "Actor Object Reference") (OtherComp :type "PrimitiveComponent Object Reference") (OtherBodyIndex :type Integer) (bFromSweep :type Boolean) (SweepResult :type "HitResult Structure (by ref)"))
  (bind _as_default_pawn_bp (`self.As Default Pawn BP`))
  (`PrimitiveComponent.SetCollisionEnabled` (`self.NoGoodLeft`) "NoCollision")
  (`PrimitiveComponent.SetCollisionEnabled` (`self.NoGoodRight`) "NoCollision")
  (`PrimitiveComponent.SetCollisionEnabled` (`self.CollisionComponent`) "NoCollision")
  (`ActorComponent.Deactivate` (`self.NoGoodLeft`))
  (`ActorComponent.Deactivate` OverlappedComponent)
  (`ActorComponent.Deactivate` (`self.NoGoodRight`))
  (`ActorComponent.Deactivate` (`self.CollisionComponent`))
  (bind _asfootball_blueprint (cast `/Game/Blueprints/Football_Blueprint` OtherActor))
  (if (not (`/Game/Blueprints/Football_Blueprint.FgHitGround` _asfootball_blueprint))
    (set `/Game/Blueprints/Football_Blueprint.FgNoGood` true _asfootball_blueprint)
    (`|SpawnActorFromClass` "/Game/Blueprints/Football/NoGoodMark.NoGoodMark_C" (`KismetMathLibrary.MakeTransform` (`self.K2_GetActorLocation` OtherActor)) "Undefined" "OverrideRootScale" null null)
    (bind _output_get (set `self.Streak` 1))
    (set `/Game/Blueprints/DefaultPawn_BP.Streak` _output_get _as_default_pawn_bp)
    (`self.DecreaseBalls`)
    (`/Game/Blueprints/EndlessUI.SetFooballs` (`/Game/Blueprints/DefaultPawn_BP.UI` _as_default_pawn_bp))
    (`KismetSystemLibrary.Delay` 2.0)
    (`/Game/Blueprints/Football_Blueprint.Reset` _asfootball_blueprint)))

(event `self.NoGoodRight.OnComponentBeginOverlap`
  (params (OverlappedComponent :type "PrimitiveComponent Object Reference") (OtherActor :type "Actor Object Reference") (OtherComp :type "PrimitiveComponent Object Reference") (OtherBodyIndex :type Integer) (bFromSweep :type Boolean) (SweepResult :type "HitResult Structure (by ref)"))
  (bind _as_default_pawn_bp (`self.As Default Pawn BP`))
  (`PrimitiveComponent.SetCollisionEnabled` (`self.NoGoodRight`) "NoCollision")
  (`PrimitiveComponent.SetCollisionEnabled` (`self.NoGoodLeft`) "NoCollision")
  (`PrimitiveComponent.SetCollisionEnabled` (`self.CollisionComponent`) "NoCollision")
  (`ActorComponent.Deactivate` (`self.NoGoodRight`))
  (`ActorComponent.Deactivate` OverlappedComponent)
  (`ActorComponent.Deactivate` (`self.NoGoodLeft`))
  (`ActorComponent.Deactivate` (`self.CollisionComponent`))
  (bind _asfootball_blueprint (cast `/Game/Blueprints/Football_Blueprint` OtherActor))
  (if (not (`/Game/Blueprints/Football_Blueprint.FgHitGround` _asfootball_blueprint))
    (set `/Game/Blueprints/Football_Blueprint.FgNoGood` true _asfootball_blueprint)
    (`|SpawnActorFromClass` "/Game/Blueprints/Football/NoGoodMark.NoGoodMark_C" (`KismetMathLibrary.MakeTransform` (`self.K2_GetActorLocation` OtherActor)) "Undefined" "OverrideRootScale" null null)
    (bind _output_get (set `self.Streak` 1))
    (set `/Game/Blueprints/DefaultPawn_BP.Streak` _output_get _as_default_pawn_bp)
    (`self.DecreaseBalls`)
    (`/Game/Blueprints/EndlessUI.SetFooballs` (`/Game/Blueprints/DefaultPawn_BP.UI` _as_default_pawn_bp))
    (`KismetSystemLibrary.Delay` 2.0)
    (`/Game/Blueprints/Football_Blueprint.Reset` _asfootball_blueprint)))

(fn `DecreaseBalls`
  (bind _asendless_game_mode (`self.GetEndlessGameMode`))
  (bind _result (`/Engine/EditorBlueprintResources/StandardMacros.DecrementInt` (`EndlessGameMode.GetFootballsLeft` _asendless_game_mode))
    (:`  `
      (`EndlessGameMode.SetFootballsLeft` _asendless_game_mode _result)
      (`KismetSystemLibrary.PrintString` (`KismetStringLibrary.Conv_IntToString` (`EndlessGameMode.GetFootballsLeft` _asendless_game_mode))))))

(fn `IncreaseScore`
  (bind _streak (`self.Streak`))
  (bind _asendless_game_mode (`self.GetEndlessGameMode`))
  (`EndlessGameMode.SetDifficulty` _asendless_game_mode (+ (`EndlessGameMode.GetDifficulty` _asendless_game_mode) 1))
  (bind _returnvalue (`EndlessGameMode.IncrementScore` _asendless_game_mode (* (`self.FG_Good_ScoreAmount`) (`self.Streak`))))
  (`EndlessGameMode.SetScore` _asendless_game_mode _returnvalue)
  (if (< _streak 5)
    (`/Engine/EditorBlueprintResources/StandardMacros.IncrementInt` _streak
      (:`  `
        _)))
  (set `/Game/Blueprints/DefaultPawn_BP.Streak` (`self.Streak`) (`self.As Default Pawn BP`))
  (bind _asdefault_pawn_bp (cast `/Game/Blueprints/DefaultPawn_BP` (`GameplayStatics.GetPlayerPawn` 0)))
  (bind _returnvalue_2 (`EndlessGameMode.GetScore` _asendless_game_mode))
  (if (>= _returnvalue_2 (`/Game/Blueprints/DefaultPawn_BP.HighScore` _asdefault_pawn_bp))
    (bind _returnvalue_3 (`EndlessGameMode.SetHighScore` _asendless_game_mode _returnvalue_2))
    (`KismetSystemLibrary.PrintString` (`KismetStringLibrary.Conv_IntToString` _returnvalue_3) true true (struct :`R` 1.0 :`B` 0.795874 :`A` 1.0))
    (bind _returnvalue_4 (`GameplayStatics.DoesSaveGameExist` (`self.SlotName`)))
    (if _returnvalue_4
      (bind _returnvalue_5 (`GameplayStatics.LoadGameFromSlot` (`self.SlotName`)))
      (bind _output_get (set `self.SaveSubClass` _returnvalue_5))
      (bind _asscore_save (cast `/Game/Blueprints/ScoreSave` _output_get))
      (bind _output_get_2 (set `/Game/Blueprints/ScoreSave.HighScore` _returnvalue_3 _asscore_save))
      (bind _asdefault_pawn_bp_2 (cast `/Game/Blueprints/DefaultPawn_BP` (`GameplayStatics.GetPlayerPawn` 0)))
      (set `/Game/Blueprints/DefaultPawn_BP.HighScore` _output_get_2 _asdefault_pawn_bp_2)
      (`GameplayStatics.SaveGameToSlot` (`self.SaveSubClass`) (`self.SlotName`))
      (else
        (bind _returnvalue_6 (`GameplayStatics.CreateSaveGameObject` "/Game/Blueprints/ScoreSave.ScoreSave_C"))
        (bind _output_get_3 (set `self.SaveSubClass` _returnvalue_6))
        (bind _asscore_save_2 (cast `/Game/Blueprints/ScoreSave` _output_get_3))
        (bind _output_get_4 (set `/Game/Blueprints/ScoreSave.HighScore` _returnvalue_3 _asscore_save_2))
        (bind _asdefault_pawn_bp_3 (cast `/Game/Blueprints/DefaultPawn_BP` (`GameplayStatics.GetPlayerPawn` 0)))
        (set `/Game/Blueprints/DefaultPawn_BP.HighScore` _output_get_4 _asdefault_pawn_bp_3)
        (`GameplayStatics.SaveGameToSlot` (`self.SaveSubClass`) (`self.SlotName`))))))

(fn `SetDifficultyLimit`
  (bind _as_endless_game_mode (`self.As Endless Game Mode`))
  (bind _as_endless_game_mode_2 (`self.As Endless Game Mode`))
  (if (== (- (`EndlessGameMode.GetDifficulty` _as_endless_game_mode_2) (`EndlessGameMode.GetDifficultyFloor` _as_endless_game_mode_2)) 10)
    (`EndlessGameMode.SetDifficultyFloor` _as_endless_game_mode (+ (`EndlessGameMode.GetDifficultyFloor` _as_endless_game_mode) 5))
    (`KismetSystemLibrary.PrintString` "RESET NEW LIMIT")))

(fn `UserConstructionScript`)